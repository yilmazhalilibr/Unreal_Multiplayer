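; BP_PC_Core is a core player controller that manages an in-game menu and switches input focus between gameplay and UI.
; It starts in game-only input, and the Toggle GameMenu action shows or collapses the menu.
; The GM_GameMenu widget is created lazily on first toggle and then reused.
; FocusWidget shows the cursor with Game And UI input focused on the menu, while FocusGame reverses this.
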(event `self.ReceiveBeginPlay`
  (`WidgetBlueprintLibrary.SetInputMode_GameOnly` self))

(event `InputAction|Toggle GameMenu`
  (params (Key :type "Key Structure"))
  (:`Pressed`
    (`self.ToggleGameMenu`)))

(fn `FocusGame`
  (set `self.bShowMouseCursor` false)
  (`WidgetBlueprintLibrary.SetInputMode_GameOnly` self))

(fn `FocusWidget`
  (set `self.bShowMouseCursor` true)
  (`WidgetBlueprintLibrary.SetInputMode_GameAndUIEx` self (`self.WB_GameMenu`)))

(fn `ToggleGameMenu`
  (`self.WB_GameMenu`
    (:`then`
      (if (`Widget.IsVisible` (`self.WB_GameMenu`))
        (`Widget.SetVisibility` (`self.WB_GameMenu`) "Collapsed")
        (`self.FocusGame`)
        (return)
        (else
          (`Widget.SetVisibility` (`self.WB_GameMenu`) "Visible")
          (`self.FocusWidget`)
          (return))))
    (:`else`
      (bind _returnvalue (`|CreateWidget` "/Game/Widgets/GameWidgets/GM_GameMenu.GM_GameMenu_C" self))
      (bind _output_get (set `self.WB_GameMenu` _returnvalue))
      (`UserWidget.AddToViewport` _output_get 0)
      (`self.FocusWidget`)
      (return))))

(fn `UserConstructionScript`)